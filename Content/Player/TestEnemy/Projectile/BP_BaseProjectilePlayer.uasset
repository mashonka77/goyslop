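; Base player projectile that damages enemies on contact.
; Its Box overlap casts to BaseEnemy and, unless the enemy is in one excluded state, applies BaseDamage with the DT_Proj damage type, crediting the projectile's owner as causer.
; A hit spawns an emitter at the enemy's location and destroys the projectile.
; A similar static-mesh impact branch exists but never runs, so that overlap handler ignores non-enemy actors.
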(event OnComponentBeginOverlap(Box)
  (params (OverlappedComponent :type Primitive%20Component%20Object%20Reference) (OtherActor :type Actor%20Object%20Reference) (OtherComp :type Primitive%20Component%20Object%20Reference) (OtherBodyIndex :type Integer) (bFromSweep :type Boolean) (SweepResult :type Hit%20Result%20Structure%20%28by%20ref%29))
  (bind _asbase_enemy (Utilities|Casting|CastToBaseEnemy OtherActor))
  (if (Utilities|Enum|NotEqual(Enum) (Default|GetState _asbase_enemy) "NewEnumerator3")
    (Game|Damage|ApplyDamage _asbase_enemy (Variables|Default|GetBase%20Damage) 0 (Components|GetOwner) "/Game/DamageSystem/DamageTypes/DT_Proj.DT_Proj_C")
    (Effects|SpawnEmitteratLocation 0 (Transformation|GetActorLocation _asbase_enemy))
    (Actor|DestroyActor)))

(event EventBeginPlay)

(event Collision|EventActorBeginOverlap
  (params (OtherActor :type Actor%20Object%20Reference)))

(event EventTick
  (params (DeltaSeconds :type Float%20%28single-precision%29)))

(fn ConstructionScript)