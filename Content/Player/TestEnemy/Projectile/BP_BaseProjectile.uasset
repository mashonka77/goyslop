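; Base enemy projectile Blueprint that damages the player on contact through its Box overlap.
; It hits BP_Player only when the player's frames check is off and the player is not in one excluded state, applying DT_Proj damage credited to the projectile's owner.
; A player hit or an overlap with an exact StaticMeshActor spawns an emitter at that actor's location and destroys the projectile.
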(event OnComponentBeginOverlap(Box)
  (params (OverlappedComponent :type Primitive%20Component%20Object%20Reference) (OtherActor :type Actor%20Object%20Reference) (OtherComp :type Primitive%20Component%20Object%20Reference) (OtherBodyIndex :type Integer) (bFromSweep :type Boolean) (SweepResult :type Hit%20Result%20Structure%20%28by%20ref%29))
  (bind _asbp_player (Utilities|Casting|CastToBP_Player OtherActor)
    (:then
      (if (and (not (Default|AreFramesEnabled? _asbp_player)) (Utilities|Enum|NotEqual(Enum) (Default|GetState _asbp_player) "NewEnumerator3"))
        (Game|Damage|ApplyDamage _asbp_player (Variables|Default|GetBase%20Damage) 0 (Components|GetOwner) "/Game/DamageSystem/DamageTypes/DT_Proj.DT_Proj_C")
        (Utilities|IsValid _asbp_player
          (:Is%20Valid
            (Effects|SpawnEmitteratLocation 0 (Transformation|GetActorLocation _asbp_player)))
          (:Is%20Not%20Valid
            _))
        (Actor|DestroyActor)))
    (:CastFailed
      (if (== (Utilities|GetClass OtherActor) "/Script/Engine.StaticMeshActor")
        (Effects|SpawnEmitteratLocation 0 (Transformation|GetActorLocation OtherActor))
        (Actor|DestroyActor)))))

(event EventBeginPlay)

(event Collision|EventActorBeginOverlap
  (params (OtherActor :type Actor%20Object%20Reference)))

(event EventTick
  (params (DeltaSeconds :type Float%20%28single-precision%29)))

(fn ConstructionScript)