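; BP_Spawner is a trigger volume that spawns enemies once, when BP_Player first overlaps its box.
; It reads an Enemies map of class to count, spawning each at random navigable points within Radius of itself.
; Each spawned actor is yawed to face the player, and each player overlap draws a temporary debug sphere showing the radius.
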(event OnComponentBeginOverlap(Box)
  (params (OverlappedComponent :type Primitive%20Component%20Object%20Reference) (OtherActor :type Actor%20Object%20Reference) (OtherComp :type Primitive%20Component%20Object%20Reference) (OtherBodyIndex :type Integer) (bFromSweep :type Boolean) (SweepResult :type Hit%20Result%20Structure%20%28by%20ref%29))
  (Utilities|Casting|CastToBP_Player OtherActor)
  (Variables|Default|SetPlayer OtherActor)
  (CallFunction|Spawn)
  (Rendering|Debug|DrawDebugSphere (Transformation|GetActorLocation) (Variables|Default|GetRadius) 18 "(R=1.000000,G=0.000000,B=0.283896,A=1.000000)" 1e+01 3.0))

(event Custom|Spawn
  (bind _enemies (Variables|Default|GetEnemies))
  (Utilities|FlowControl|DoOnce false
    (:Completed
      (bind _keys (Utilities|Map|Keys _enemies))
      (for _array_element _keys
        (for _index (range 1 (.Value (Utilities|Map|Find _enemies _array_element)))
          (bind _randomlocation (Class|NavigationSystemV1|GetRandomLocationinNavigableRadius (Transformation|GetActorLocation) (Variables|Default|GetRadius) 0 0))
          (bind _returnvalue (Game|SpawnActorfromClass _array_element (Math|Transform|MakeTransform _randomlocation "0, 0, 0" "1.000000,1.000000,1.000000") "AdjustIfPossibleButAlwaysSpawn" "MultiplyWithRoot" 0 0))
          (Transformation|SetActorRotation _returnvalue (Math|Rotator|MakeRotator (.roll (Transformation|GetActorRotation _returnvalue)) (.pitch (Transformation|GetActorRotation _returnvalue)) (.yaw (Math|Rotator|FindLookatRotation (Transformation|GetActorLocation _returnvalue) (Transformation|GetActorLocation (Variables|Default|GetPlayer)))))))))))

(event EventBeginPlay)

(event Collision|EventActorBeginOverlap
  (params (OtherActor :type Actor%20Object%20Reference)))

(event EventTick
  (params (DeltaSeconds :type Float%20%28single-precision%29)))

(fn ConstructionScript)