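; Combo component that keeps a style meter, ranking StylePoints from D to SSS by fixed thresholds.
; A looping timer lowers points once enough time has passed since LastHitTime, then updates the rank; GetRankProgress returns normalized progress within it.
; RegisterSuccessfulHit looks up DT_ComboAttacks to count repeated attack tags, but neither adds points nor sets LastHitTime.
; The OnComboUpdated broadcast is unconnected.
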(event Custom|DecayCombo
  (if (>= (- (Utilities|Time|GetGameTimeinSeconds) (Variables|Default|GetLast%20Hit%20Time)) (Variables|Default|GetDecay%20Delay))
    (Variables|Default|SetStyle%20Points (Math|Float|Max(Float) (- (Variables|Default|GetStyle%20Points) (Variables|Default|GetDecay%20Step)) 0.0))
    (CallFunction|UpdateRank)))

(event EventBeginPlay
  (bind _returnvalue (Utilities|Time|SetTimerbyEvent (delegate Custom|DecayCombo) (Variables|Default|GetDecay%20Interval) true))
  (Variables|Default|SetDecayTimerHandle _returnvalue))

(event EventTick
  (params (DeltaSeconds :type Float%20%28single-precision%29)))

(fn NewFunction)

(fn RegisterSuccessfulHit
  (params (AttackTag :type Gameplay%20Tag%20Structure) (OptionalBonusMultiplier :type Float%20%28double-precision%29) (RowName :type Name))
  (bind _returnvalue (Utilities|GetDataTableRow "/Game/CombatSystem/DT_ComboAttacks.DT_ComboAttacks" RowName)
    (:then
      (if (== (Variables|Default|GetLast%20Attack%20Tag) (.AttackTag (Utilities|Struct|BreakST_ComboAttackData _returnvalue)))
        (Variables|Default|SetRepeat%20Count (+ (Variables|Default|GetRepeat%20Count) 1))
        (else
          (Variables|Default|SetRepeat%20Count 0)
          (Variables|Default|SetLast%20Attack%20Tag (.AttackTag (Utilities|Struct|BreakST_ComboAttackData _returnvalue))))))))

(fn UpdateRank
  (if (< (Variables|Default|GetStyle%20Points) 5e+02)
    (Variables|Default|SetCurrent%20Rank "NewEnumerator0")
    (elif (< (Variables|Default|GetStyle%20Points) 1.2e+03)
      (Variables|Default|SetCurrent%20Rank "NewEnumerator1")
      (elif (< (Variables|Default|GetStyle%20Points) 2e+03)
        (Variables|Default|SetCurrent%20Rank "NewEnumerator2")
        (elif (< (Variables|Default|GetStyle%20Points) 3e+03)
          (Variables|Default|SetCurrent%20Rank "NewEnumerator3")
          (elif (< (Variables|Default|GetStyle%20Points) 4e+03)
            (Variables|Default|SetCurrent%20Rank "NewEnumerator4")
            (elif (< (Variables|Default|GetStyle%20Points) 5e+03)
              (Variables|Default|SetCurrent%20Rank "NewEnumerator5")
              (elif (>= (Variables|Default|GetStyle%20Points) 5e+03)
                (Variables|Default|SetCurrent%20Rank "NewEnumerator6")))))))))

(fn GetRankProgress
  (bind _current_rank (Variables|Default|GetCurrent%20Rank))
  (bind _returnvalue (Utilities|Select :Index _current_rank :NewEnumerator0 0.0 :NewEnumerator1 5e+02 :NewEnumerator2 1.2e+03 :NewEnumerator3 2e+03 :NewEnumerator4 3e+03 :NewEnumerator5 4e+03 :NewEnumerator6 5e+03))
  (return (Math|Float|Clamp(Float) (/ (- (Variables|Default|GetStyle%20Points) _returnvalue) (- (Utilities|Select :Index _current_rank :NewEnumerator0 5e+02 :NewEnumerator1 1.2e+03 :NewEnumerator2 2e+03 :NewEnumerator3 3e+03 :NewEnumerator4 4e+03 :NewEnumerator5 5e+03 :NewEnumerator6 6e+03) _returnvalue)))))